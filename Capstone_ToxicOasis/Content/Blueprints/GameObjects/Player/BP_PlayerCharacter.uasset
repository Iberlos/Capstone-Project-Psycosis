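; Player character Blueprint that manages the main HUD, pause menu and health percentage.
; BeginPlay adds HUD_Main, and the Pause input flip-flops between opening PauseMenu with a cursor and clearing all widgets to rebuild the HUD and PreAlpha widget.
; Tick computes HealthPercent from the health component, and two helper functions toggle mouse cursor and input mode.
; InitiateFadefromBlack is empty, and the StartBlack level sequence logic is disconnected.
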(event EventInitiateFadefromBlack
  (params (a_targetPlayer :type Player%20Character%20Object%20Reference)))

(event EventBeginPlay
  ;[1 1 1] Making HUD ref
  (bind _returnvalue (UserInterface|CreateWidget "/Game/Blueprints/UI/HUD_Main.HUD_Main_C"))
  (bind _output_get (Variables|Default|SetHUDREF _returnvalue))
  (UserInterface|Viewport|AddtoViewport _output_get 0))

(event EventTick
  (params (DeltaSeconds :type Float%20%28single-precision%29))
  ;[1 1 1] Setting up health percent var
  (bind _returnvalue (Class|MyCharacter|GetHealthComponent))
  (bind _returnvalue_2 (Class|ObjectHealthComponent|GetHealth _returnvalue))
  (bind _returnvalue_3 (Class|ObjectHealthComponent|GetMaxHealth _returnvalue))
  (Variables|Default|SetHealthPercent (/ _returnvalue_2 _returnvalue_3)))

(event Input|ActionEvents|InputActionPause
  (params (Key :type Key%20Structure :default "None"))
  (bind _returnvalue (Game|GetPlayerController 0))
  (bind _returnvalue_2 (Game|GetPlayerController 0))
  ;[1 1 1] PauseGame
  (:Pressed
    (Utilities|FlowControl|FlipFlop
      (:A
        (Game|SetGamePaused true)
        (bind _returnvalue_3 (UserInterface|CreateWidget "/Game/Blueprints/GameInstance/PauseMenu.PauseMenu_C" _returnvalue_2))
        (UserInterface|Viewport|AddtoViewport _returnvalue_3 0)
        (Input|SetInputModeGameandUI _returnvalue_2 0 "DoNotLock" false)
        (Variables|/Script/Engine.PlayerController|SetbShowMouseCursor _returnvalue_2 true))
      (:B
        (Game|SetGamePaused false)
        (Viewport|RemoveAllWidgets)
        (Input|SetInputModeGameOnly _returnvalue)
        (bind _returnvalue_4 (UserInterface|CreateWidget "/Game/Blueprints/GameInstance/Pre-Alpha.Pre-Alpha_C"))
        (UserInterface|Viewport|AddtoViewport _returnvalue_4 0)
        (bind _returnvalue_5 (UserInterface|CreateWidget "/Game/Blueprints/UI/HUD_Main.HUD_Main_C"))
        (bind _output_get (Variables|Default|SetHUDREF _returnvalue_5))
        (UserInterface|Viewport|AddtoViewport _output_get 0)
        (Variables|/Script/Engine.PlayerController|SetbShowMouseCursor _returnvalue false)))))

(fn ConstructionScript)

(fn EnableMouseCursor
  (bind _returnvalue (Game|GetPlayerController 0))
  (Input|SetInputModeGameandUI _returnvalue (Variables|Default|GetHUDREF) "DoNotLock" true)
  (Variables|/Script/Engine.PlayerController|SetbShowMouseCursor _returnvalue true))

(fn DisableMouseCursor
  (bind _returnvalue (Game|GetPlayerController 0))
  (Input|SetInputModeGameOnly _returnvalue)
  (Variables|/Script/Engine.PlayerController|SetbShowMouseCursor _returnvalue false))