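; Game instance for the Capstone game that manages multiplayer sessions through host, join and destroy events on the first player controller.
; HOST creates an advanced session with the given connection, LAN and extra settings, then opens the chosen level as a listen server.
; Successful HOST and JOIN calls set a multiplayer-active flag by casting the game instance to its own class.
; DESTROY ends the session without clearing that flag.
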(event Custom|HOST
  (params (PublicConnections :type Integer) (bUseLAN :type Boolean) (ExtraSettings :type Array%20of%20Session%20Property%20Key%20Pair%20Structures) (LevelName :type Name))
  ;[1 1 1] HOSTSession
  (bind _output_get (Variables|Default|SetLevelName LevelName))
  (|AdvancedSession ExtraSettings (Game|GetPlayerController 0) PublicConnections 0 bUseLAN true false true true false false false true
    (:OnSuccess
      (Game|OpenLevel(byName) _output_get false "listen")
      (bind _asbp_capstone_game_instance (Utilities|Casting|CastToBP_CapstoneGameInstance (Game|GetGameInstance)))
      (Class|CapstoneGameInstance|SetMutltiplayerActive _asbp_capstone_game_instance true))))

(event Custom|JOIN
  (params (SearchResult :type Blueprint%20Session%20Result%20Structure%20%28by%20ref%29))
  ;[1 1 1] JOINSession
  (|JoinSession (Game|GetPlayerController 0) SearchResult
    (:OnSuccess
      (bind _asbp_capstone_game_instance (Utilities|Casting|CastToBP_CapstoneGameInstance (Game|GetGameInstance)))
      (Class|CapstoneGameInstance|SetMutltiplayerActive _asbp_capstone_game_instance true))))

(event Custom|DESTROY
  ;[1 1 1] DESTROYSession
  (|DestroySession (Game|GetPlayerController 0)))