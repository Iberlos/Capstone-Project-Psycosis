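; Lamppost Blueprint for environmental dressing, with a spotlight that can flicker.
; On BeginPlay, if Flicker is set, a looping Delay sets the SpotLight to a random intensity within a min/max range.
; Each wait between changes is also randomized between DelayMin and DelayMax, and the construction script is empty.
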(event EventBeginPlay
  (if (Variables|Default|GetFlicker)
    (Rendering|Components|Light|SetIntensity (Variables|Default|GetSpotLight) (Math|Random|RandomFloatinRange (Variables|Default|GetIntensity_Min) (Variables|Default|GetIntensity_Max)) :!label _label)
    (Utilities|FlowControl|Delay (Math|Random|RandomFloatinRange (Variables|Default|GetDelay_Min) (Variables|Default|GetDelay_Max)))
    (goto _label)))

(fn ConstructionScript)