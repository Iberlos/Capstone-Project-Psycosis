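; BP_FallBackTrigger is an overlap trigger that recovers characters entering it, returning players to the level and removing AI.
; For a player with a valid HUD, it fades to black, waits briefly, calls FallBackIntoLevel, then ends the fade.
; AI characters go back to their owning spawner's pool, or are destroyed when they have no valid spawner.
; An authority switch remains in the graph but never runs.
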(event Collision|EventActorBeginOverlap
  (params (OtherActor :type Actor%20Object%20Reference))
  (bind _asbp_player_character (Utilities|Casting|CastToBP_PlayerCharacter OtherActor)
    (:then
      (bind _output_get (Variables|Default|SetLastPlayerRef _asbp_player_character))
      (if (Utilities|IsValid (Variables|/Game/Blueprints/GameObjects/Player/BP_PlayerCharacter.BP_PlayerCharacter_C|GetHUDREF _output_get))
        (Default|StartFadetoBlack (Variables|/Game/Blueprints/GameObjects/Player/BP_PlayerCharacter.BP_PlayerCharacter_C|GetHUDREF _output_get) (Variables|Default|GetLastPlayerRef))
        (Utilities|FlowControl|Delay 1.0)
        (Class|PlayerCharacter|FallBackIntoLevel (Variables|Default|GetLastPlayerRef))
        (Default|EndFadetoBlack (Variables|/Game/Blueprints/GameObjects/Player/BP_PlayerCharacter.BP_PlayerCharacter_C|GetHUDREF _output_get) (Variables|Default|GetLastPlayerRef))))
    (:CastFailed
      (bind _asaibase_character (Utilities|Casting|CastToAIBaseCharacter OtherActor))
      (bind _returnvalue (Class|AIBaseCharacter|GetOwningSpawner _asaibase_character))
      (if (Utilities|IsValid _returnvalue)
        (Class|AISpawner|SendBacktoPool _returnvalue _asaibase_character)
        (else
          (Actor|DestroyActor _asaibase_character))))))

(fn ConstructionScript)