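; Moving platform actor that travels along a spline, optionally starting on BeginPlay.
; A timeline scaled by Time lerps distance along the spline to set the platform's relative location.
; The authority records timeline time in CurrentTime, and remotes call SetNewTime when their timeline drifts from it beyond a tolerance.
; A rotator timeline is present but never runs.
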(event Custom|StartMoving
  ;[1 1 1] Start Moving
  (Components|Timeline|SetPlayRate (Variables|Default|GetPlatformMover) (/ 1.0 (Variables|Default|GetTime)))
  (bind (_direction _alpha _time) (Timeline|PlatformMover Play)
    (:Update
      (Variables|Default|SetAlpha _alpha)
      (Utilities|FlowControl|Sequence
        (:then_0
          (Transformation|SetRelativeLocationAndRotation (Variables|Default|GetMovingPlatform) (Spline|GetLocationatDistanceAlongSpline (Variables|Default|GetSpline) (Math|Float|Lerp 0.0 (Spline|GetSplineLength (Variables|Default|GetSpline)) (Variables|Default|GetAlpha)) "Local") "0, 0, 0" false false))
        (:then_1
          (Networking|SwitchHasAuthority
            (:Authority
              (Variables|Default|SetCurrentTime _time))))))))

(event EventBeginPlay
  ;[1 1 1] BeginPlay StartMoving
  (if (Variables|Default|GetMovePlatformOnBeginPlay)
    (CallFunction|StartMoving)))

(event EventTick
  (params (DeltaSeconds :type Float%20%28single-precision%29))
  (Networking|SwitchHasAuthority
    (:Remote
      (if (not (Math|Float|NearlyEqual(Float) (stale _time) (Variables|Default|GetCurrentTime) 0.5))
        ;[1 1 1] Start Moving
        (bind (_direction _alpha _time) (Timeline|PlatformMover SetNewTime)
          (:Update
            (Variables|Default|SetAlpha _alpha)
            (Utilities|FlowControl|Sequence
              (:then_0
                (Transformation|SetRelativeLocationAndRotation (Variables|Default|GetMovingPlatform) (Spline|GetLocationatDistanceAlongSpline (Variables|Default|GetSpline) (Math|Float|Lerp 0.0 (Spline|GetSplineLength (Variables|Default|GetSpline)) (Variables|Default|GetAlpha)) "Local") "0, 0, 0" false false))
              (:then_1
                (Networking|SwitchHasAuthority
                  (:Authority
                    (Variables|Default|SetCurrentTime _time)))))))))))

(fn ConstructionScript)